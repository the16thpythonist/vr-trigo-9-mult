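; BPCube is an actor that toggles between its assembled position and an exploded, spread-out position each time its Explode event is called.
; The first call saves its location and jumps it outward along the vector from its MyCenter BPCone, doubling that distance.
; If the cast to BPCone fails, its own world location serves as the offset.
; The next call snaps it back to the saved location, with no interpolation.
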(event `self.ReceiveBeginPlay`)

(event `Explode`
  (if (`self.bIsExploded`)
    (`self.K2_SetActorLocation` (`self.OriginalLocation`))
    (set `self.bIsExploded` false)
    (else
      (`|ExecutionSequence`
        (:`then_0`
          (set `self.OriginalLocation` (`self.K2_GetActorLocation`)))
        (:`then_1`
          (bind _asbpcone (cast `/Game/Blueprints/BPCone` (`self.MyCenter`))
            (:`then`
              (set `self.MovingDirection` (- (`self.K2_GetActorLocation`) (`self.K2_GetActorLocation` _asbpcone))))
            (:`CastFailed`
              (set `self.MovingDirection` (`self.K2_GetActorLocation`)))))
        (:`then_2`
          (`self.K2_SetActorLocation` (+ (`self.K2_GetActorLocation`) (* (`self.MovingDirection`) 1.0)))
          (set `self.bIsExploded` true))))))

(fn `UserConstructionScript`)