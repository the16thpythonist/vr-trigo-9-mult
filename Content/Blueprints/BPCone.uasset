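; BPCone is an input-driven trigger actor that detonates every BPCube in the level.
; Pressing N or the left motion controller shoulder gathers all BPCube actors with GetAllActorsOfClass and calls Explode on each.
; Releasing N only prints a debug message.
; Several unconnected cast and name-printing nodes remain unused, and the construction script is empty.
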(event `Key|X`
  (params (Key :type "Key Structure" :default "AnyKey")))

(event `Key|N`
  (params (Key :type "Key Structure" :default "AnyKey"))
  (:`Pressed`
    (bind _outactors (`GameplayStatics.GetAllActorsOfClass` "/Game/Blueprints/BPCube.BPCube_C" :!label _label))
    (for _array_element _outactors
      (`/Game/Blueprints/BPCube.Explode` _array_element)))
  (:`Released`
    (`KismetSystemLibrary.PrintText` "BPCone-N-released -----")))

(event `Key|MotionController_Left_Shoulder`
  (params (Key :type "Key Structure" :default "AnyKey"))
  (:`Pressed`
    (goto _label)))

(event `Key|C`
  (params (Key :type "Key Structure" :default "AnyKey")))

(fn `UserConstructionScript`)