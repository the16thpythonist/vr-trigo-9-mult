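; 1BPCone2 is a cone actor that serves as a keyboard-driven test and debug trigger for 1BPCube2 actors.
; Pressing X finds every 1BPCube2 in the level and calls Explode on each.
; Pressing C prints the names of those cubes, and releasing it prints the cone's center of mass, component world location and actor location.
; The cast to BPCube and a SetActorLocation node are unconnected leftovers.
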(event `Key|X`
  (params (Key :type "Key Structure" :default "AnyKey"))
  (:`Pressed`
    (bind _outactors (`GameplayStatics.GetAllActorsOfClass` "/Game/Blueprints/1BPCube2.1BPCube2_C"))
    (for _array_element _outactors
      (`/Game/Blueprints/1BPCube2.Explode` _array_element))))

(event `Key|C`
  (params (Key :type "Key Structure" :default "AnyKey"))
  (:`Pressed`
    (`KismetSystemLibrary.PrintString` "C-Pressed")
    (bind _outactors (`GameplayStatics.GetAllActorsOfClass` "/Game/Blueprints/1BPCube2.1BPCube2_C"))
    (for _array_element _outactors
      (`KismetSystemLibrary.PrintText` (`KismetTextLibrary.Conv_StringToText` (`KismetSystemLibrary.GetObjectName` _array_element)))))
  (:`Released`
    (`KismetSystemLibrary.PrintString` "Center of mass cone:")
    (bind _returnvalue (`PrimitiveComponent.GetCenterOfMass` (`self.Cone`) "None"))
    (`KismetSystemLibrary.PrintString` "Center of mass cone:")
    (`KismetSystemLibrary.PrintString` (`KismetStringLibrary.Conv_VectorToString` _returnvalue))
    (`KismetSystemLibrary.PrintString` "Location cone:")
    (`KismetSystemLibrary.PrintString` (`KismetStringLibrary.Conv_VectorToString` (`SceneComponent.K2_GetComponentLocation` (`self.Cone`))))
    (`KismetSystemLibrary.PrintString` "location self (Actor)::")
    (`KismetSystemLibrary.PrintString` (`KismetStringLibrary.Conv_VectorToString` (`self.K2_GetActorLocation`)))))

(fn `UserConstructionScript`)