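; 1BPCube2 is a cube part that toggles between its place and an exploded-view position, and can be grabbed by a motion controller.
; Explode saves the current location and pushes the cube away from its MyCenter 1BPCone2 by their offset, doubling the distance; the next call restores that location.
; Pickup attaches the root to the controller's component and Drop detaches it, keeping world transforms with physics simulation off throughout.
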(event `self.ReceiveBeginPlay`
  (`|ExecutionSequence`
    (:`then_0`
      (set `self.OriginalLocation` (`self.K2_GetActorLocation`)))
    (:`then_1`
      (`PrimitiveComponent.SetSimulatePhysics` (`self.StaticMeshComponent`) false))))

(event `Explode`
  (if (`self.bIsExploded`)
    (`self.K2_SetActorLocation` (`self.OriginalLocation`))
    (set `self.bIsExploded` false)
    (else
      (`|ExecutionSequence`
        (:`then_0`
          (set `self.OriginalLocation` (`self.K2_GetActorLocation`)))
        (:`then_1`
          ;[1 1 1] Class of Center
          (bind _as1bpcone_2 (cast `/Game/Blueprints/1BPCone2` (`self.MyCenter`))
            (:`then`
              (set `self.MovingDirection` (- (`self.K2_GetActorLocation`) (`self.K2_GetActorLocation` _as1bpcone_2))))
            (:`CastFailed`
              (set `self.MovingDirection` (`self.K2_GetActorLocation`)))))
        (:`then_2`
          (`self.K2_SetActorLocation` (+ (`self.K2_GetActorLocation`) (* (`self.MovingDirection`) 1.0)))
          (set `self.bIsExploded` true))))))

(event `/Game/VirtualRealityBP/Blueprints/PickupActorInterface.Pickup`
  (params (AttachTo :type "SceneComponent Object Reference"))
  (`PrimitiveComponent.SetSimulatePhysics` (`self.StaticMeshComponent`) false)
  (`SceneComponent.K2_AttachToComponent` (`self.K2_GetRootComponent`) AttachTo "None" "KeepWorld" "KeepWorld" "KeepWorld" false))

(event `/Game/VirtualRealityBP/Blueprints/PickupActorInterface.Drop`
  (`PrimitiveComponent.SetSimulatePhysics` (`self.StaticMeshComponent`) false)
  (`self.K2_DetachFromActor` "KeepWorld" "KeepWorld" "KeepWorld"))

(fn `UserConstructionScript`)